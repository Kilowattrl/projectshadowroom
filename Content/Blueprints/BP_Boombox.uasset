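; BP_Boombox is a boombox prop that a VR button switches on and off.
; When the button state changes to on, it activates the audio component and plays a timeline; when off, it deactivates the audio and stops the timeline.
; The timeline drives the roll of a secondary static mesh, keeping its pitch and yaw, so that part turns while the boombox plays.
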(event OnButtonStateChanged(VRButton)
  (params (ButtonState :type Boolean) (InteractingActor :type Actor%20Object%20Reference) (InteractingComponent :type Primitive%20Component%20Object%20Reference))
  (bind _audio (Variables|Default|GetAudio))
  (if ButtonState
    (Components|Activation|Activate _audio false)
    (CallFunction|ActivateTurny)
    (else
      (Components|Activation|Deactivate _audio)
      (CallFunction|DeactivateTurny))))

(event Custom|ActivateTurny
  (bind _staticmesh2 (Variables|Default|GetStaticMesh2))
  (bind _relativerotation (Variables|/Script/Engine.SceneComponent|GetRelativeRotation _staticmesh2))
  (bind _newtrack_0 (Timeline|TurnyTime Play)
    (:Update
      (Transformation|SetRelativeRotation _staticmesh2 (Math|Rotator|MakeRotator _newtrack_0 (.pitch _relativerotation) (.yaw _relativerotation)) false false))))

(event Custom|DeactivateTurny
  (bind _staticmesh2 (Variables|Default|GetStaticMesh2))
  (bind _relativerotation (Variables|/Script/Engine.SceneComponent|GetRelativeRotation _staticmesh2))
  (bind _newtrack_0 (Timeline|TurnyTime Stop)
    (:Update
      (Transformation|SetRelativeRotation _staticmesh2 (Math|Rotator|MakeRotator _newtrack_0 (.pitch _relativerotation) (.yaw _relativerotation)) false false))))

(fn ConstructionScript)