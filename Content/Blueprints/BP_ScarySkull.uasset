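; BP_ScarySkull is a one-shot scare actor, triggered when a component tagged "interact" overlaps its sphere.
; It activates audio, then chained timelines move and roll the skull before opening its jaw while shaking it.
; Eye and jaw particles precede a vanish effect that scales the skull and particle system.
; Finally, it sends an electrical-state-on message to the Electrical reference and destroys itself.
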(event OnComponentBeginOverlap(SphereCollision)
  (params (OverlappedComponent :type Primitive%20Component%20Object%20Reference) (OtherActor :type Actor%20Object%20Reference) (OtherComp :type Primitive%20Component%20Object%20Reference) (OtherBodyIndex :type Integer) (bFromSweep :type Boolean) (SweepResult :type Hit%20Result%20Structure%20%28by%20ref%29))
  (bind _defaultsceneroot (Variables|Default|GetDefaultSceneRoot))
  (bind _vanishparticlesystem (Variables|Default|GetVanishParticleSystem))
  (bind _defaultsceneroot_2 (Variables|Default|GetDefaultSceneRoot))
  (bind _vanishparticlesystem_2 (Variables|Default|GetVanishParticleSystem))
  (bind _jaw (Variables|Default|GetJaw))
  (bind _defaultsceneroot_3 (Variables|Default|GetDefaultSceneRoot))
  (bind _returnvalue (Transformation|GetWorldRotation _defaultsceneroot))
  (bind _relativerotation (Variables|/Script/Engine.SceneComponent|GetRelativeRotation _defaultsceneroot_2))
  (bind _relativelocation (Variables|/Script/Engine.SceneComponent|GetRelativeLocation _vanishparticlesystem_2))
  (bind _relativerotation_2 (Variables|/Script/Engine.SceneComponent|GetRelativeRotation _jaw))
  ;[1 1 1] Overlap Sphere / Trigger Event
  (if (Components|ComponentHasTag OtherComp "interact")
    (Utilities|FlowControl|DoOnce false
      (:Completed
        (Utilities|FlowControl|Sequence
          (:then_0
            (Components|Activation|Activate (Variables|Default|GetAudio) false))
          (:then_1
            ;[1 1 1] Initial Upwards Movement
            (bind _newtrack_0 (Timeline|SkullMovement Play)
              (:Update
                (Transformation|SetWorldLocation _defaultsceneroot (+ (* _newtrack_0 8.5) (Transformation|GetWorldLocation _defaultsceneroot)) false false))
              (:Finished
                (bind _rotation (Timeline|SkullRotation Play)
                  (:Update
                    (Transformation|SetWorldRotation _defaultsceneroot (Math|Rotator|MakeRotator (+ (* _rotation 2.0) (.roll _returnvalue)) (.pitch _returnvalue) (.yaw _returnvalue)) false false))
                  (:Finished
                    ;[1 1 1] Jaw Open and Skull Shake
                    (Utilities|FlowControl|Sequence
                      (:then_0
                        (bind _newtrack_0_2 (Timeline|JawRotation Play)
                          (:Update
                            (Transformation|SetRelativeRotation _jaw (Math|Rotator|MakeRotator _newtrack_0_2 (.pitch _relativerotation_2) (.yaw _relativerotation_2)) false false))
                          (:Finished
                            (Components|Activation|Activate (Variables|Default|GetRightEyeParticleSystem) false)
                            (Components|Activation|Activate (Variables|Default|GetLeftEyeParticleSystem) false)
                            (Components|Activation|Activate (Variables|Default|GetJawParticleSystem) false)
                            (Utilities|FlowControl|Delay 1.8)
                            (Components|Activation|Activate (Variables|Default|GetVanishParticleSystem) false)
                            (Utilities|FlowControl|Delay 0.2)
                            ;[1 1 1] Particle and scale down and kill
                            (Utilities|FlowControl|Sequence
                              (:then_0
                                (bind (_direction _scale _location) (Timeline|VanishParticleScale Play)
                                  (:Update
                                    (Transformation|SetRelativeScale3D _defaultsceneroot_3 (* (Variables|/Script/Engine.SceneComponent|GetRelativeScale3D _defaultsceneroot_3) _scale))
                                    (Transformation|SetRelativeLocation _vanishparticlesystem_2 (Math|Vector|MakeVector (.x _relativelocation) (* _location -1e+02) (.z _relativelocation)) false false))))
                              (:then_1
                                (Utilities|FlowControl|Delay 0.3)
                                (bind _newtrack_1 (Timeline|VanishSkullScale Play)
                                  (:Update
                                    (Transformation|SetRelativeScale3D _vanishparticlesystem (* (Variables|/Script/Engine.SceneComponent|GetRelativeScale3D _vanishparticlesystem) _newtrack_1)))
                                  (:Finished
                                    (Class|ElectricalObject|CurrentStateChange(Message) (Variables|Default|GetElectrical%20) 0 true 0.0)
                                    (Actor|DestroyActor))))))))
                      (:then_1
                        (bind (_direction_2 _shake _tilt) (Timeline|SkullShake Play)
                          (:Update
                            (Transformation|SetRelativeRotation _defaultsceneroot_2 (Math|Rotator|MakeRotator (+ _tilt (.roll _relativerotation)) _shake (.yaw _relativerotation)) false false)))))))))))))))

(event EventBeginPlay
  ;[1 1 1] Overlap Sphere / Trigger Event
)

(fn ConstructionScript)