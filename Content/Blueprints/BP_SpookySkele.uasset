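; BP_SpookySkele is a spooky prop that advances along a spline only while the player is not looking at it.
; CurrentStateChange starts a looping timer that waits until the mesh is first rendered, then toggles movement using WasRecentlyRendered.
; The Movement timeline plays when the mesh is unseen and stops when seen, setting mesh location and rotation from spline distance with a yaw offset.
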(event Custom|Move
  (bind _spline (Variables|Default|GetSpline))
  ;[1 1 1] Movement Timeline
  (bind _time (Timeline|Movement Play)
    (:Update
      ;[1 1 1] Set World Location and Rotation
      (Transformation|SetWorldLocationAndRotation (Variables|Default|GetStaticMesh) (.location (Spline|GetTransformatDistanceAlongSpline _spline (* _time (Spline|GetSplineLength _spline)) "World" false)) (Math|Rotator|CombineRotators "0,-90.000000, 0" (.rotation (Spline|GetTransformatDistanceAlongSpline _spline (* _time (Spline|GetSplineLength _spline)) "World" false))) false false))))

(event Custom|Check
  (bind _staticmesh (Variables|Default|GetStaticMesh))
  (bind _returnvalue (Class|PrimitiveComponent|WasRecentlyRendered _staticmesh 0.3))
  ;[1 1 1] Check if recently rendered
  (if (Variables|Default|GetHasBeenSeenByPlayer)
    ;[1 1 1] Move or pause movement
    (if _returnvalue
      (CallFunction|Pause)
      (else
        (CallFunction|Move)))
    (else
      (Variables|Default|SetHasBeenSeenByPlayer _returnvalue))))

(event Custom|Pause
  (bind _spline (Variables|Default|GetSpline))
  ;[1 1 1] Movement Timeline
  (bind _time (Timeline|Movement Stop)
    (:Update
      ;[1 1 1] Set World Location and Rotation
      (Transformation|SetWorldLocationAndRotation (Variables|Default|GetStaticMesh) (.location (Spline|GetTransformatDistanceAlongSpline _spline (* _time (Spline|GetSplineLength _spline)) "World" false)) (Math|Rotator|CombineRotators "0,-90.000000, 0" (.rotation (Spline|GetTransformatDistanceAlongSpline _spline (* _time (Spline|GetSplineLength _spline)) "World" false))) false false))))

(event EventCurrentStateChange
  (params (CurrentProvider :type Object%20Object%20Reference) (ElectricalState :type Boolean) (CurrentFlow :type Float%20%28single-precision%29))
  ;[1 1 1] Timer Activation
  (Utilities|Time|SetTimerbyEvent (delegate Custom|Check) 0.3 true))

(fn ConstructionScript)