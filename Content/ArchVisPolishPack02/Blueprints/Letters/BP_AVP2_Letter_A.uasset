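; Alphabet letter actor that disappears when a component tagged "Interact" overlaps its sphere.
; The construction script picks one of the A-Z meshes from the LetterMesh variable and creates a dynamic alphabet material instance on it.
; On overlap it activates StaticSizzle and plays a timeline that drives the material's Appearance parameter, then destroys itself when the timeline finishes.
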(event OnComponentBeginOverlap(Sphere)
  (params (OverlappedComponent :type Primitive%20Component%20Object%20Reference) (OtherActor :type Actor%20Object%20Reference) (OtherComp :type Primitive%20Component%20Object%20Reference) (OtherBodyIndex :type Integer) (bFromSweep :type Boolean) (SweepResult :type Hit%20Result%20Structure%20%28by%20ref%29))
  (if (Components|ComponentHasTag OtherComp "Interact")
    (Components|Activation|Activate (Variables|Default|GetStaticSizzle) false)
    (bind _disapear (Timeline|Timeline_0 Play)
      (:Update
        (Rendering|Material|SetScalarParameterValue (Variables|Default|GetMID_Alphabet) "Appearance" (Math|Float|Lerp 0.0 1e+01 _disapear) :!class /Script/Engine.MaterialInstanceDynamic))
      (:Finished
        (Actor|DestroyActor)))))

(fn ConstructionScript
  (bind _returnvalue (Rendering|Material|CreateDynamicMaterialInstance (Variables|Default|GetStaticMesh) 0 "/Game/ArchVisPolishPack02/Materials/M_AVP2_Alphabet.M_AVP2_Alphabet" "None" :!class /Script/Engine.PrimitiveComponent))
  (Variables|Default|SetMID_Alphabet _returnvalue)
  (Components|StaticMesh|SetStaticMesh (Variables|Default|GetStaticMesh) (Utilities|Select :Index (Variables|Default|GetLetterMesh) :NewEnumerator0 "/Game/ArchVisPolishPack02/Meshes/Letters/SM_AVP2_A.SM_AVP2_A" :NewEnumerator1 "/Game/ArchVisPolishPack02/Meshes/Letters/SM_AVP2_B.SM_AVP2_B" :NewEnumerator2 "/Game/ArchVisPolishPack02/Meshes/Letters/SM_AVP2_C.SM_AVP2_C" :NewEnumerator3 "/Game/ArchVisPolishPack02/Meshes/Letters/SM_AVP2_D.SM_AVP2_D" :NewEnumerator4 "/Game/ArchVisPolishPack02/Meshes/Letters/SM_AVP2_E.SM_AVP2_E" :NewEnumerator5 "/Game/ArchVisPolishPack02/Meshes/Letters/SM_AVP2_F.SM_AVP2_F" :NewEnumerator6 "/Game/ArchVisPolishPack02/Meshes/Letters/SM_AVP2_G.SM_AVP2_G" :NewEnumerator7 "/Game/ArchVisPolishPack02/Meshes/Letters/SM_AVP2_H.SM_AVP2_H" :NewEnumerator8 "/Game/ArchVisPolishPack02/Meshes/Letters/SM_AVP2_I.SM_AVP2_I" :NewEnumerator9 "/Game/ArchVisPolishPack02/Meshes/Letters/SM_AVP2_J.SM_AVP2_J" :NewEnumerator10 "/Game/ArchVisPolishPack02/Meshes/Letters/SM_AVP2_K.SM_AVP2_K" :NewEnumerator11 "/Game/ArchVisPolishPack02/Meshes/Letters/SM_AVP2_L.SM_AVP2_L" :NewEnumerator12 "/Game/ArchVisPolishPack02/Meshes/Letters/SM_AVP2_M.SM_AVP2_M" :NewEnumerator13 "/Game/ArchVisPolishPack02/Meshes/Letters/SM_AVP2_N.SM_AVP2_N" :NewEnumerator14 "/Game/ArchVisPolishPack02/Meshes/Letters/SM_AVP2_O.SM_AVP2_O" :NewEnumerator15 "/Game/ArchVisPolishPack02/Meshes/Letters/SM_AVP2_P.SM_AVP2_P" :NewEnumerator16 "/Game/ArchVisPolishPack02/Meshes/Letters/SM_AVP2_Q.SM_AVP2_Q" :NewEnumerator17 "/Game/ArchVisPolishPack02/Meshes/Letters/SM_AVP2_R.SM_AVP2_R" :NewEnumerator18 "/Game/ArchVisPolishPack02/Meshes/Letters/SM_AVP2_S.SM_AVP2_S" :NewEnumerator19 "/Game/ArchVisPolishPack02/Meshes/Letters/SM_AVP2_T.SM_AVP2_T" :NewEnumerator20 "/Game/ArchVisPolishPack02/Meshes/Letters/SM_AVP2_U.SM_AVP2_U" :NewEnumerator21 "/Game/ArchVisPolishPack02/Meshes/Letters/SM_AVP2_V.SM_AVP2_V" :NewEnumerator22 "/Game/ArchVisPolishPack02/Meshes/Letters/SM_AVP2_W.SM_AVP2_W" :NewEnumerator23 "/Game/ArchVisPolishPack02/Meshes/Letters/SM_AVP2_X.SM_AVP2_X" :NewEnumerator24 "/Game/ArchVisPolishPack02/Meshes/Letters/SM_AVP2_Y.SM_AVP2_Y" :NewEnumerator25 "/Game/ArchVisPolishPack02/Meshes/Letters/SM_AVP2_Z.SM_AVP2_Z")))